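; Actor that sets up warp meshes for a three-screen LED display, apparently for nDisplay rendering.
; On BeginPlay it assigns the centre, left and right LED mesh components to the matching viewports through the API's AssignWarpMeshToViewport, using Root as the shared origin.
; Overlap, Tick and the construction script are empty.
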(event `self.ReceiveBeginPlay`
  ;[1 1 1] Setup warp
  (`PicpProjectionBlueprintAPI.AssignWarpMeshToViewport` (`PicpProjectionIBlueprintLib.GetAPI`) "vp_centre" (`self.LED_Centre`) (`self.root`))
  (`PicpProjectionBlueprintAPI.AssignWarpMeshToViewport` (`PicpProjectionIBlueprintLib.GetAPI`) "vp_left" (`self.LED_Left`) (`self.root`))
  (`PicpProjectionBlueprintAPI.AssignWarpMeshToViewport` (`PicpProjectionIBlueprintLib.GetAPI`) "vp_right" (`self.LED_Right`) (`self.root`)))

(fn `UserConstructionScript`)